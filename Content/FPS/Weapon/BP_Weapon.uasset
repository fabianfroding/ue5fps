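; Weapon Blueprint that plays the cosmetic effects of a shot through its FireEffects event, skipped on dedicated servers.
; It picks the first or third-person mesh and reads the muzzle socket location.
; Helper actors for weapon fire, impacts and decals spawn on first use, attach to that mesh, and are reused with fresh impact data each shot.
; The fire sound and montage play last.
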(event `self.FireEffects`
  (params (ImpactPoint :type "Vector Structure (by ref)") (ImpactNormal :type "Vector Structure (by ref)") (ImpactSurfaceType :type "EPhysicalSurface Enum" :default "SurfaceType_Default") (bIsFirstPerson :type Boolean))
  (set `self.bIsFirstPerson` bIsFirstPerson)
  (if (not (`KismetSystemLibrary.IsDedicatedServer`))
    (set `self.ImpactPoints` (`|MakeArray` ImpactPoint))
    (set `self.ImpactNormals` (`|MakeArray` ImpactNormal))
    (set `self.ImpactSurfaceTypes` (`|MakeArray` ImpactSurfaceType))
    (`|ExecutionSequence`
      (:`then_0`
        (set `self.SkeletalMesh` (select `bool` (`self.bIsFirstPerson`) :`false` (`self.Mesh3P`) :`true` (`self.Mesh1P`))))
      (:`then_1`
        (set `self.MuzzlePosition` (`SceneComponent.GetSocketLocation` (`self.SkeletalMesh`) (`self.MuzzleSocketName`))))
      (:`then_2`
        (`|ExecutionSequence`
          (:`then_0`
            ; Reuse spawned weapon fire object
            (`/Engine/EditorBlueprintResources/StandardMacros.IsValid` (`self.WeaponFire`)
              (:`Is Valid`
                _)
              (:`Is Not Valid`
                (bind _returnvalue (`|SpawnActorFromClass` "/Game/Effects/Blueprints/B_WeaponFire.B_WeaponFire_C" (`KismetMathLibrary.MakeTransform` (0.0 0.0 0.0)) "Undefined" "OverrideRootScale" null (`self.SkeletalMesh`) true (`self.ShellEjectSystem`) true (`self.MuzzleFlashSystem`) true (`self.TracerSystem`) (`self.ShellEjectMesh`) null))
                (bind _output_get (set `self.WeaponFire` _returnvalue))
                (`self.K2_AttachToComponent` _output_get (`self.SkeletalMesh`) "None" "KeepRelative" "KeepRelative" "KeepRelative" true)))
            (set `/Game/Effects/Blueprints/B_WeaponFire.ImpactPositions` (`self.ImpactPoints`) (`self.WeaponFire`))
            (set `/Game/Effects/Blueprints/B_WeaponFire.ImpactNormals` (`self.ImpactNormals`) (`self.WeaponFire`))
            (set `/Game/Effects/Blueprints/B_WeaponFire.ImpactSurfaceTypes` (`self.ImpactSurfaceTypes`) (`self.WeaponFire`))
            (`/Game/Effects/Blueprints/B_WeaponFire.Fire` (`self.WeaponFire`) (`self.bIsFirstPerson`)))
          (:`then_1`
            ; Impact effects
            (`/Engine/EditorBlueprintResources/StandardMacros.IsValid` (`self.WeaponImpacts`)
              (:`Is Valid`
                _)
              (:`Is Not Valid`
                (bind _returnvalue_2 (`|SpawnActorFromClass` "/Game/Effects/Blueprints/B_WeaponImpacts.B_WeaponImpacts_C" (`KismetMathLibrary.MakeTransform` (0.0 0.0 0.0)) "Undefined" "OverrideRootScale" null 500.0 null))
                (bind _output_get_2 (set `self.WeaponImpacts` _returnvalue_2))
                (`self.K2_AttachToComponent` _output_get_2 (`self.SkeletalMesh`) "None" "KeepRelative" "KeepRelative" "KeepRelative" true)))
            (set `/Game/Effects/Blueprints/B_WeaponImpacts.ImpactPositions` (`self.ImpactPoints`) (`self.WeaponImpacts`))
            (set `/Game/Effects/Blueprints/B_WeaponImpacts.Sorted Impact Normals` (`self.ImpactNormals`) (`self.WeaponImpacts`))
            (set `/Game/Effects/Blueprints/B_WeaponImpacts.ImpactSurfaceTypes` (`self.ImpactSurfaceTypes`) (`self.WeaponImpacts`))
            (set `/Game/Effects/Blueprints/B_WeaponImpacts.MuzzlePosition` (`self.MuzzlePosition`) (`self.WeaponImpacts`))
            (`/Game/Effects/Blueprints/B_WeaponImpacts.Fire` (`self.WeaponImpacts`) (`self.bIsFirstPerson`)))
          (:`then_2`
            ; Weapon decals
            (`/Engine/EditorBlueprintResources/StandardMacros.IsValid` (`self.WeaponDecals`)
              (:`Is Valid`
                _)
              (:`Is Not Valid`
                (bind _returnvalue_3 (`|SpawnActorFromClass` "/Game/Effects/Blueprints/B_WeaponDecals.B_WeaponDecals_C" (`KismetMathLibrary.MakeTransform` (0.0 0.0 0.0)) "Undefined" "MultiplyWithRoot" null null))
                (bind _output_get_3 (set `self.WeaponDecals` _returnvalue_3))
                (`self.K2_AttachToComponent` _output_get_3 (`self.SkeletalMesh`) "None" "KeepRelative" "KeepRelative" "KeepRelative" true)))
            (set `/Game/Effects/Blueprints/B_WeaponDecals.ImpactPositions` (`self.ImpactPoints`) (`self.WeaponDecals`))
            (set `/Game/Effects/Blueprints/B_WeaponDecals.ImpactNormals` (`self.ImpactNormals`) (`self.WeaponDecals`))
            (set `/Game/Effects/Blueprints/B_WeaponDecals.Impact Surface Types` (`self.ImpactSurfaceTypes`) (`self.WeaponDecals`))
            (`/Game/Effects/Blueprints/B_WeaponDecals.fire` (`self.WeaponDecals`) (`self.MuzzlePosition`)))
          (:`then_3`
            (`GameplayStatics.PlaySoundAtLocation` (`self.WeaponFireSound`) (`self.K2_GetActorLocation`) (struct) 1.0 1.0 0.0 null null null null)
            (`|PlayMontage` (`self.SkeletalMesh`) (`self.WeaponFireMontage`))))))))

(fn `UserConstructionScript`)
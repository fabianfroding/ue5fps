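; BP_ShooterCharacter is the FPS shooter character Blueprint, handling aim zoom and death animation.
; On aim, a timeline blends the first-person camera FOV from the default to the current weapon's aim FOV from the combat component, reversing when aiming stops.
; On death effects, it plays a random montage from its death montage list on the mesh, if any exist.
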(event `self.OnAim`
  (params (bIsAiming :type Boolean))
  (if bIsAiming
    (bind (_direction _alpha) (`Timeline|AimTimeline` :!label _label)
      (:`Update`
        (`CameraComponent.SetFieldOfView` (`self.FirstPersonCamera`) (`KismetMathLibrary.Lerp` (`self.DefaultFOV`) (`Weapon.AimFOV` (`CombatComponent.CurrentWeapon` (`self.CombatComponent`))) _alpha))))
    (else
      (goto _label :!via `Reverse`))))

(event `self.DeathEffects`
  (bind _deathmontages (`self.DeathMontages`))
  (if (not (`KismetArrayLibrary.Array_IsEmpty` _deathmontages))
    (`|PlayMontage` (`self.Mesh`) (`KismetArrayLibrary.Array_Random` _deathmontages))))

(fn `UserConstructionScript`)